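; BP_Bonus_Ball is a bonus ball actor that travels and bounces until it overlaps a KillZVolume, which destroys it.
; BeginPlay randomizes the X of its Direction, keeps Y and zeroes Z.
; Each tick moves it by a swept world offset scaled by Speed and delta time, without physics simulation.
; A blocking hit replaces Direction with a reflection computed from the surface normal's X and Y.
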(event `self.ReceiveActorBeginOverlap`
  (params (OtherActor :type "Actor Object Reference"))
  (cast `KillZVolume` OtherActor)
  (`self.K2_DestroyActor`))

(event `self.ReceiveBeginPlay`
  (bind (_direction_x _direction_y) (`KismetMathLibrary.BreakVector` (`self.Direction`)))
  (bind _output_get (set `self.Direction` (`KismetMathLibrary.MakeVector` (`KismetMathLibrary.RandomFloatInRange` -100.0 100.0) _direction_y)))
  (bind _sweephitresult (`self.K2_AddActorWorldOffset` self (* (* _output_get (`self.Speed`)) (stale `self.ReceiveTick` DeltaSeconds)) true false :!label _label))
  (bind (_bblockinghit _binitialoverlap _time _distance _location _impactpoint _normal) (`GameplayStatics.BreakHitResult` _sweephitresult))
  (if _bblockinghit
    (set `self.Direction` (`KismetMathLibrary.GetReflectionVector` (`self.Direction`) (`KismetMathLibrary.MakeVector` (.x _normal) (.y _normal))))))

(event `self.ReceiveTick`
  (params (DeltaSeconds :type "Float (single-precision)"))
  (goto _label))

(fn `UserConstructionScript`)