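; BP_Bonus is a moving bonus pickup that BP_Pawn collects by overlapping it.
; Each tick it moves by Direction and Speed with a swept world offset.
; On overlap with BP_Pawn it spawns a BP_Bonus_Ball at its capsule's location and destroys itself.
; Ending an overlap with a KillZVolume also destroys it, and both outcomes print a Russian message.
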(event `self.ReceiveActorEndOverlap`
  (params (OtherActor :type "Actor Object Reference"))
  (cast `KillZVolume` OtherActor)
  (`self.K2_DestroyActor`)
  (`KismetSystemLibrary.PrintString` "Ой, а кто это потерял бонус?" true true (struct :`R` 1.0 :`B` 0.093626 :`A` 1.0)))

(event `self.ReceiveTick`
  (params (DeltaSeconds :type "Float (single-precision)"))
  (`self.K2_AddActorWorldOffset` self (* (* (`self.Direction`) (`self.Speed`)) DeltaSeconds) true false))

(event `self.ReceiveActorBeginOverlap`
  (params (OtherActor :type "Actor Object Reference"))
  (bind _returnvalue_location (`KismetMathLibrary.BreakTransform` (`SceneComponent.K2_GetComponentToWorld` (`self.Capsule_Bonus`))))
  (cast `/Game/BP_Class/BP_Pawn` OtherActor)
  (`|SpawnActorFromClass` "/Game/BP_Class/BP_Bonus_Ball.BP_Bonus_Ball_C" (`KismetMathLibrary.MakeTransform` _returnvalue_location) "AdjustIfPossibleButAlwaysSpawn" "OverrideRootScale" null null)
  (`self.K2_DestroyActor`)
  (`KismetSystemLibrary.PrintString` "Бонусы сюда!" true true (struct :`R` 0.432794 :`G` 1.0 :`B` 0.581629 :`A` 1.0)))

(fn `UserConstructionScript`)