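; BP_healthSystem is a Blueprint that tracks a health point value for its owner or user.
; AddHealths and SubHealths change the value by one through UpateHealths, which prints the new value to screen and stores it without clamping.
; IsDeath reports whether health is at or below zero, and the event graph holds no active logic.
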(fn `AddHealths`
  (`self.Upate Healths` (+ (`self.HealthPoints`) 1)))

(fn `IsDeath`
  (returns (ReturnValue :type Boolean))
  (return (<= (`self.HealthPoints`) 0)))

(fn `Sub Healths`
  (`self.Upate Healths` (- (`self.HealthPoints`) 1)))

(fn `Upate Healths`
  (params (HealthPoints :type Integer))
  (`KismetSystemLibrary.PrintString` (`KismetStringLibrary.Conv_IntToString` HealthPoints))
  (set `self.HealthPoints` HealthPoints))