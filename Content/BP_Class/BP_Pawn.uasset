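; BP_Pawn is a player pawn that moves sideways and manages ball spawning and lives.
; MoveRight input shifts it along X in fixed, swept steps that do not scale with frame time.
; SpawnBall, called on BeginPlay, deducts health first, then either prints game over or spawns a BP_Ball at the capsule and binds to its OnDead event.
; A separate DoOnce first-spawn graph is not called here.
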(event `InputAxis|MoveRight`
  (params (AxisValue :type "Float (single-precision)"))
  (if (> AxisValue 0.0)
    (`self.K2_AddActorWorldOffset` (50.0 0.0 0.0) true)))

(event `InputAxis|MoveRight`
  (params (AxisValue :type "Float (single-precision)"))
  (if (< AxisValue 0.0)
    (`self.K2_AddActorWorldOffset` (-50.0 0.0 0.0) true)))

(event `self.ReceiveBeginPlay`
  (`self.SpawnBall`))

(fn `SpawnBall`
  (bind _bp_healthsystem (`self.BP_healthSystem`))
  (bind _returnvalue_location (`KismetMathLibrary.BreakTransform` (`SceneComponent.K2_GetComponentToWorld` (`self.Capsule`))))
  (`/Game/BP_Class/BP_healthSystem.Sub Healths` _bp_healthsystem)
  (if (`/Game/BP_Class/BP_healthSystem.IsDeath` _bp_healthsystem)
    (`KismetSystemLibrary.PrintString` "Game OVER!")
    (else
      (bind _returnvalue (`|SpawnActorFromClass` "/Game/BP_Class/BP_Ball.BP_Ball_C" (`KismetMathLibrary.MakeTransform` _returnvalue_location) "AdjustIfPossibleButAlwaysSpawn" "OverrideRootScale" null null))
      (bind _output_get (set `self.BP_Ball` _returnvalue))
      (add `/Game/BP_Class/BP_Ball.On dead` _output_get (`|CreateDelegate` :!event `SpawnBall`)))))

(fn `UserConstructionScript`)

(fn `Первый спавн мячика`
  (bind _returnvalue_location (`KismetMathLibrary.BreakTransform` (`SceneComponent.K2_GetComponentToWorld` (`self.Capsule`))))
  (`/Engine/EditorBlueprintResources/StandardMacros.DoOnce` false
    (:`Completed`
      (`|SpawnActorFromClass` "/Game/BP_Class/BP_Ball.BP_Ball_C" (`KismetMathLibrary.MakeTransform` _returnvalue_location) "AdjustIfPossibleButAlwaysSpawn" "OverrideRootScale" null null))))